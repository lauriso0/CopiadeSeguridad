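; AI-controlled father character that periodically heads to the girl's room and can cause the player's defeat.
; IniciarTimer shows a countdown widget, starts a looping one-second timer and plays a delayed sound.
; At zero, the countdown resets and writes the room location and a flag to the AI controller's Blackboard, which ResetGoToRoom clears.
; Capsule contact with the player while they hold an object shows the defeat screen and pauses the game.
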(event `IniciarTimer`
  (bind _returnvalue (`|CreateWidget` "/Game/Widgets/WBP_FatherTImer.WBP_FatherTImer_C"))
  (set `self.FatherTimerWidget` _returnvalue)
  (bind _outactors (`GameplayStatics.GetAllActorsOfClass` "/Game/Blueprints/BP_GirlRoom.BP_GirlRoom_C"))
  (set `self.GirlRoomRef` (`|GetArrayItem` _outactors))
  (`KismetSystemLibrary.K2_SetTimer` self "UpdateTimer" 1.0 true)
  (`UserWidget.AddToViewport` _returnvalue 0)
  (`KismetSystemLibrary.Delay` 35.0)
  (`GameplayStatics.PlaySound2D` "/Game/Sounds/SBP_PAPAHIJA.SBP_PAPAHIJA" 1.0 1.0 0.0 null null))

(event `self.ReceiveBeginPlay`)

(event `self.CapsuleComponent.OnComponentHit`
  (params (HitComponent :type "PrimitiveComponent Object Reference") (OtherActor :type "Actor Object Reference") (OtherComp :type "PrimitiveComponent Object Reference") (NormalImpulse :type "Vector Structure") (Hit :type "HitResult Structure (by ref)"))
  (bind _asbp_first_person_character (cast `/Game/FirstPerson/Blueprints/BP_FirstPersonCharacter` OtherActor))
  (if (`KismetSystemLibrary.IsValid` (`/Game/FirstPerson/Blueprints/BP_FirstPersonCharacter.heldObject` _asbp_first_person_character))
    (bind _returnvalue (`|CreateWidget` "/Game/Widgets/WBP_DerrotaPapa.WBP_DerrotaPapa_C"))
    (`UserWidget.AddToViewport` _returnvalue 0)
    (`GameplayStatics.SetGamePaused` true)
    (set `PlayerController.bShowMouseCursor` true (`GameplayStatics.GetPlayerController` 0))))

(fn `GoToGirlRoom`
  (bind _asbp_father_aicontroller (cast `/Game/Blueprints/BP_FatherAIController` (`self.GetController` self)))
  (bind _returnvalue (`AIBlueprintHelperLibrary.GetBlackboard` _asbp_father_aicontroller))
  (`BlackboardComponent.SetValueAsBool` _returnvalue "bGoingToRoom" true)
  (`BlackboardComponent.SetValueAsVector` _returnvalue "GirlRoomLocation" (`SceneComponent.K2_GetComponentLocation` (`/Game/Blueprints/BP_GirlRoom.RoomZone` (`self.GirlRoomRef`)))))

(fn `ResetGoToRoom`
  (set `self.bIsGoingToRoom` false)
  (bind _asbp_father_aicontroller (cast `/Game/Blueprints/BP_FatherAIController` (`self.GetController` self)))
  (`BlackboardComponent.SetValueAsBool` (`AIBlueprintHelperLibrary.GetBlackboard` _asbp_father_aicontroller) "bGoingToRoom" false))

(fn `UpdateTimer`
  (set `self.TimerCount` (- (`self.TimerCount`) 1.0))
  (if (<= (`self.TimerCount`) 0.0)
    (set `self.TimerCount` 90.0)
    (set `self.bIsGoingToRoom` true)
    (`self.GoToGirlRoom`)
    (else
      (bind _aswbp_father_timer (cast `/Game/Widgets/WBP_FatherTImer` (`self.FatherTimerWidget`)))
      (set `TextBlock.Text` (`|FormatText` "El padre viene en: {time}" (`KismetStringLibrary.Conv_StringToDouble` (`KismetStringLibrary.Conv_DoubleToString` (`self.TimerCount`)))) (`/Game/Widgets/WBP_FatherTImer.TimerText` _aswbp_father_timer)))))

(fn `UserConstructionScript`)