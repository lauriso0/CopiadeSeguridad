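; Enemy pawn that chases the first-person player and triggers the defeat screen when it catches them.
; Pawn sensing writes a non-hiding player to the AI controller's blackboard and sets a short timer to LoseSight, which clears those keys so it returns to patrolling.
; A capsule hit on a non-hiding player shows the defeat widget, pauses the game and enables the mouse cursor.
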(event `self.PawnSensor.OnSeePawn`
  (params (Pawn :type "Pawn Object Reference"))
  ; Perseguir
  (bind _asbp_first_person_character (cast `/Game/FirstPerson/Blueprints/BP_FirstPersonCharacter` Pawn))
  (if (not (`/Game/FirstPerson/Blueprints/BP_FirstPersonCharacter.bIsHiding` _asbp_first_person_character))
    (bind _asbp_enemy_aicontroller (cast `/Game/Blueprints/BP_EnemyAIController` (`self.GetController` self)))
    (bind _returnvalue (`AIBlueprintHelperLibrary.GetBlackboard` _asbp_enemy_aicontroller))
    (`BlackboardComponent.SetValueAsObject` _returnvalue "TargetPlayer" Pawn)
    (`BlackboardComponent.SetValueAsBool` _returnvalue "CanSeePlayer" true)
    (`KismetSystemLibrary.K2_SetTimer` self "LoseSight" 3.0)))

(event `self.CapsuleComponent.OnComponentHit`
  (params (HitComponent :type "PrimitiveComponent Object Reference") (OtherActor :type "Actor Object Reference") (OtherComp :type "PrimitiveComponent Object Reference") (NormalImpulse :type "Vector Structure") (Hit :type "HitResult Structure (by ref)"))
  ; cDerrota cuando la amante la atrapa
  (bind _asbp_first_person_character (cast `/Game/FirstPerson/Blueprints/BP_FirstPersonCharacter` OtherActor))
  (if (not (`/Game/FirstPerson/Blueprints/BP_FirstPersonCharacter.bIsHiding` _asbp_first_person_character))
    (bind _returnvalue (`|CreateWidget` "/Game/Widgets/WBP_Derrota.WBP_Derrota_C"))
    (`UserWidget.AddToViewport` _returnvalue 0)
    (`GameplayStatics.SetGamePaused` true)
    (set `PlayerController.bShowMouseCursor` true (`GameplayStatics.GetPlayerController` 0))))

(fn `LoseSight`
  ; Volver a patrullar
  (bind _asbp_enemy_aicontroller (cast `/Game/Blueprints/BP_EnemyAIController` (`self.GetController` self)))
  (bind _returnvalue (`AIBlueprintHelperLibrary.GetBlackboard` _asbp_enemy_aicontroller))
  (`BlackboardComponent.SetValueAsBool` _returnvalue "CanSeePlayer" false)
  (`BlackboardComponent.SetValueAsObject` _returnvalue "TargetPlayer" null))

(fn `UserConstructionScript`)