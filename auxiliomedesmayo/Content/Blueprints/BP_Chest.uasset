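; BP_Chest is a deposit chest that completes a room once enough carried objects are placed in it.
; Held BP_Objects overlapping ChestZone are hidden, released from the player and counted, firing deposit and room-completion dispatchers.
; CompleteRoom records progress and keys in BP_GameInstance by CurrentRoomID; its Room 4 victory-screen branch compares 0 to 4, so never runs.
; ResetChest clears the count and advances the room ID.
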(event `self.ChestZone.OnComponentBeginOverlap`
  (params (OverlappedComponent :type "PrimitiveComponent Object Reference") (OtherActor :type "Actor Object Reference") (OtherComp :type "PrimitiveComponent Object Reference") (OtherBodyIndex :type Integer) (bFromSweep :type Boolean) (SweepResult :type "HitResult Structure (by ref)"))
  ; Depositar Objeto
  (if (`KismetSystemLibrary.IsValid` OtherActor)
    (bind _asbp_object (cast `/Game/Blueprints/BP_Object` OtherActor))
    (if (`/Game/Blueprints/BP_Object.bIsHeld` _asbp_object)
      (`self.SetActorHiddenInGame` _asbp_object true)
      (`self.SetActorEnableCollision` _asbp_object false)
      (bind _asbp_first_person_character (cast `/Game/FirstPerson/Blueprints/BP_FirstPersonCharacter` (`GameplayStatics.GetPlayerCharacter` 0)))
      (set `/Game/FirstPerson/Blueprints/BP_FirstPersonCharacter.heldObject` null _asbp_first_person_character)
      (set `self.ObjectsDeposited` (+ (`self.ObjectsDeposited`) 1))
      (`self.OnObjectDeposited`)
      (if (>= (`self.ObjectsDeposited`) (`self.RequiredObjects`))
        (`self.CompleteRoom`)
        (`self.OnRoomComplete`)))))

(fn `CompleteRoom`
  (bind _asbp_game_instance (cast `/Game/Blueprints/BP_GameInstance` (`GameplayStatics.GetGameInstance`)))
  ; Room 1
  (if (== (`self.CurrentRoomID`) 1)
    (set `/Game/Blueprints/BP_GameInstance.Room1Complete` true _asbp_game_instance)
    (set `/Game/Blueprints/BP_GameInstance.KeysCollected` (+ (`/Game/Blueprints/BP_GameInstance.KeysCollected` _asbp_game_instance) 1) _asbp_game_instance)
    (else
      ; Room 2
      (if (== (`self.CurrentRoomID`) 2)
        (set `/Game/Blueprints/BP_GameInstance.Room2Complete` true _asbp_game_instance)
        (set `/Game/Blueprints/BP_GameInstance.KeysCollected` (+ (`/Game/Blueprints/BP_GameInstance.KeysCollected` _asbp_game_instance) 1) _asbp_game_instance)
        (else
          ; Room3
          (if (== (`self.CurrentRoomID`) 3)
            (set `/Game/Blueprints/BP_GameInstance.Room3Complete` true _asbp_game_instance)
            (set `/Game/Blueprints/BP_GameInstance.KeysCollected` (+ (`/Game/Blueprints/BP_GameInstance.KeysCollected` _asbp_game_instance) 1) _asbp_game_instance)
            (else
              ; Room4
              (if (== 0 4)
                (set `/Game/Blueprints/BP_GameInstance.Room4Complete` true _asbp_game_instance)
                (set `/Game/Blueprints/BP_GameInstance.KeysCollected` (+ (`/Game/Blueprints/BP_GameInstance.KeysCollected` _asbp_game_instance) 1) _asbp_game_instance)
                (bind _returnvalue (`|CreateWidget` "/Game/Widgets/WBP_Victoria.WBP_Victoria_C"))
                (`UserWidget.AddToViewport` _returnvalue 0)
                (`GameplayStatics.SetGamePaused` true)
                (set `PlayerController.bShowMouseCursor` false (`GameplayStatics.GetPlayerController` 0))))))))))

(fn `ResetChest`
  (set `self.ObjectsDeposited` 0)
  (set `self.CurrentRoomID` (+ (`self.CurrentRoomID`) 1)))

(fn `UserConstructionScript`)