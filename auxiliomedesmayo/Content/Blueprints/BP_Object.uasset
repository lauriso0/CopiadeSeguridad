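; BP_Object is an actor that can be picked up and dropped.
; PickUp disables physics on its static mesh and collision on its interaction sphere, hides the actor and flags it as held, without using the Grabber input.
; Drop unhides it, restores query-only sphere collision and clears the flag, but leaves physics simulation off.
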(event `PickUp`
  (params (Grabber :type "Actor Object Reference"))
  ; pick up and drop
  (`PrimitiveComponent.SetSimulatePhysics` (`self.StaticMesh`) false)
  (`PrimitiveComponent.SetCollisionEnabled` (`self.InteractSphere`) "NoCollision")
  (`self.SetActorHiddenInGame` true)
  (set `self.bIsHeld` true))

(event `Drop`
  ; pick up and drop
  (if (`KismetSystemLibrary.IsValid` self)
    (`self.SetActorHiddenInGame` false)
    (`PrimitiveComponent.SetCollisionEnabled` (`self.InteractSphere`) "QueryOnly")
    (set `self.bIsHeld` false)))

(fn `UserConstructionScript`)