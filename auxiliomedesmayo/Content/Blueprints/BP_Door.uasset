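; BP_Door is a room-gated door that opens once when the first-person character enters its DoorZone.
; It checks the GameInstance completion flag matching RequiredRoomID (rooms 1 to 3), printing a missing-items message if unmet.
; Opening runs a timeline that sets the pivot to a fixed rotation without interpolation.
; When the timeline finishes, every BP_Chest in the level is reset.
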(event `Open door`
  (set `self.bIsOpen` true)
  (`Timeline|DoorOpening`
    (:`Update`
      (`SceneComponent.K2_SetRelativeRotation` (`self.DoorPivot`) (struct :`Yaw` 90.0) false false))
    (:`Finished`
      (bind _outactors (`GameplayStatics.GetAllActorsOfClass` "/Game/Blueprints/BP_Chest.BP_Chest_C"))
      (for _array_element _outactors
        (bind _asbp_chest (cast `/Game/Blueprints/BP_Chest` _array_element))
        (`/Game/Blueprints/BP_Chest.ResetChest` _asbp_chest)))))

(event `self.DoorZone.OnComponentBeginOverlap`
  (params (OverlappedComponent :type "PrimitiveComponent Object Reference") (OtherActor :type "Actor Object Reference") (OtherComp :type "PrimitiveComponent Object Reference") (OtherBodyIndex :type Integer) (bFromSweep :type Boolean) (SweepResult :type "HitResult Structure (by ref)"))
  (cast `/Game/FirstPerson/Blueprints/BP_FirstPersonCharacter` OtherActor)
  (if (not (`self.bIsOpen`))
    (bind _asbp_game_instance (cast `/Game/Blueprints/BP_GameInstance` (`GameplayStatics.GetGameInstance`)))
    (if (== (`self.RequiredRoomID`) 1)
      (if (`/Game/Blueprints/BP_GameInstance.Room1Complete` _asbp_game_instance)
        (`self.Open door`)
        (else
          (`KismetSystemLibrary.PrintString` "Necesitas todos los objetos")))
      (elif (== (`self.RequiredRoomID`) 2)
        (if (`/Game/Blueprints/BP_GameInstance.Room2Complete` _asbp_game_instance)
          (`self.Open door`)
          (else
            (`KismetSystemLibrary.PrintString` "Necesitas todos los objetos")))
        (elif (== (`self.RequiredRoomID`) 3)
          (if (`/Game/Blueprints/BP_GameInstance.Room3Complete` _asbp_game_instance)
            (`self.Open door`)
            (else
              (`KismetSystemLibrary.PrintString` "Necesitas todos los objetos"))))))))

(fn `UserConstructionScript`)